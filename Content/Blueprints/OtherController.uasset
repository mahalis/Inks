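; OtherController is a controller Blueprint that makes its pawn wander randomly.
; A looping timer picks a new random horizontal direction every few seconds, starting immediately on BeginPlay.
; Tick feeds that direction into the pawn's movement input, scaled by remapped Perlin noise over game time.
; A random per-instance time offset varies the noise, so each pawn's movement strength fluctuates independently.
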(event EventBeginPlay
  (Variables|Default|SetNoiseTimeOffset (Math|Random|RandomFloatinRange 0.0 1e+02))
  (Utilities|Time|SetTimerbyFunctionName 0 "PickMovementDirection" 3.0 true)
  (CallFunction|PickMovementDirection))

(event EventTick
  (params (DeltaSeconds :type Float%20%28single-precision%29))
  (Pawn|Input|AddMovementInput (Pawn|GetControlledPawn) (Variables|Default|GetCurrentMoveDirection) (Class|KismetAnimationLibrary|MakePerlinNoiseandRemap (+ (Utilities|Time|GetGameTimeinSeconds) (Variables|Default|GetNoiseTimeOffset)) 0.2 1.0) false))

(fn ConstructionScript)

(fn PickMovementDirection
  (bind _output_get (LocalVariables|SetAngle (Math|Random|RandomFloatinRange 0.0 3.6e+02)))
  (Variables|Default|SetCurrentMoveDirection (Math|Vector|MakeVector (Math|Trig|Sin(Degrees) _output_get) (Math|Trig|Cos(Degrees) _output_get) 0.0)))