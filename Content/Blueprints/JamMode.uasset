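; Game mode for a jam game where the player consumes color-level pawns, managing title and end screens, tutorial and game over.
; After a preset tutorial wave, PopulateEnvironment tops up pawns by player level, adding enough prey to pass the nearest predator.
; At max level spawning stops, and consuming the last pawn ends the game.
; Player damage spawns a fragment with a burst effect; spawns use best-candidate disc sampling to avoid crowding.
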(event EventBeginPlay
  (bind _returnvalue (Game|GetPlayerController 0))
  (Utilities|FlowControl|Sequence
    (:then_0
      (Class|WidgetBlueprintLibrary|SetFocustoGameViewport)
      (Input|SetInputModeGameandUI _returnvalue 0 "DoNotLock" false)
      (bind _returnvalue_2 (UserInterface|CreateWidget "/Game/Blueprints/UI/TitleScreen.TitleScreen_C" _returnvalue))
      (bind _output_get (Variables|UI|SetTitleScreenWidget _returnvalue_2))
      (UserInterface|Viewport|AddtoViewport _output_get 0)
      (bind _returnvalue_3 (UserInterface|CreateWidget "/Game/Blueprints/UI/EndScreen.EndScreen_C" _returnvalue))
      (bind _output_get_2 (Variables|UI|SetEndScreenWidget _returnvalue_3))
      (UserInterface|Viewport|AddtoViewport _output_get_2 0))
    (:then_1
      (bind _outactors (Actor|GetAllActorsOfClass "/Script/Engine.CameraActor"))
      (Game|Player|SetViewTargetwithBlend (Game|GetPlayerController 0) (Utilities|Array|Get(acopy) _outactors) 0.0 "VTBlend_Linear" 0.0 false))
    (:then_2
      (bind _asjam_player_pawn (Utilities|Casting|CastToJamPlayerPawn (Game|Player|GetPlayerPawn 0)))
      (bind _output_get_3 (Variables|Default|SetPlayer _asjam_player_pawn))
      (Variables|/Game/Blueprints/JamPawnBase.JamPawnBase_C|SetMode _output_get_3 self))
    (:then_3
      (CallFunction|Reset))))

(event EventTick
  (params (DeltaSeconds :type Float%20%28single-precision%29)))

(fn ConstructionScript)

(fn Reset
  (Utilities|FlowControl|Sequence
    (:then_0
      (Variables|GameState|SetPlaying false))
    (:then_1
      (Variables|GameState|SetGameOver false))
    (:then_2
      (Widget|SetVisibility (Variables|UI|GetEndScreenWidget) "Hidden"))
    (:then_3
      (Widget|SetVisibility (Variables|UI|GetTitleScreenWidget) "Visible"))
    (:then_4
      (Default|SetColorLevel (Variables|Default|GetPlayer)))))

(fn GetScore
  (return 0))

(fn Begin
  (Variables|GameState|SetPlaying true)
  (Widget|SetVisibility (Variables|UI|GetTitleScreenWidget) "Hidden")
  (Default|SetColorLevel (Variables|Default|GetPlayer))
  (Population|SetupTutorial)
  (bind _asjam_player_controller (Utilities|Casting|CastToJamPlayerController (Game|GetPlayerController 0)))
  (Variables|/Game/Blueprints/JamPlayerController.JamPlayerController_C|SetShouldObeyUserInput _asjam_player_controller true))

(fn PopulateEnvironment
  (bind _outactors (Actor|GetAllActorsOfClass "/Game/Blueprints/JamPawnBase.JamPawnBase_C"))
  (bind _output_get (LocalVariables|SetAllPawns _outactors))
  (LocalVariables|SetClosestPredatorLevel (Variables|Constants|GetMaxColorLevel))
  (LocalVariables|SetPlayerLevel (Default|GetColorLevel (Variables|Default|GetPlayer)))
  (for _array_element _output_get
    (bind _asjam_other_pawn (Utilities|Casting|CastToJamOtherPawn _array_element))
    (if (> (Default|GetColorLevel _asjam_other_pawn) (LocalVariables|GetPlayerLevel))
      (LocalVariables|SetHasAnyPredator true)
      (LocalVariables|SetClosestPredatorLevel (Math|Integer|Min(Integer) (LocalVariables|GetClosestPredatorLevel) (Default|GetColorLevel _asjam_other_pawn)))
      (else
        (Math|Integer|IncrementInt (LocalVariables|GetAvailablePrey)))))
  (Utilities|FlowControl|Sequence
    (:then_0
      (if (LocalVariables|GetHasAnyPredator)
        (LocalVariables|SetPreyNeeded (+ (- (LocalVariables|GetClosestPredatorLevel) (LocalVariables|GetPlayerLevel)) 1))))
    (:then_1
      (LocalVariables|SetPreyNeeded (Math|Integer|Max(Integer) 0 (- (LocalVariables|GetPreyNeeded) (LocalVariables|GetAvailablePrey)))))
    (:then_2
      (LocalVariables|SetOthersToAdd (Math|Integer|Max(Integer) (- (Population|GetDesiredPopulation) (- (Utilities|Array|Length (LocalVariables|GetAllPawns)) 1)) (LocalVariables|GetPreyNeeded))))
    (:then_3
      (if (< (LocalVariables|GetPlayerLevel) (Variables|Constants|GetMaxColorLevel))
        (for _index (range 0 (- (LocalVariables|GetOthersToAdd) 1))
          (bind _location (Population|PickSpawnLocation (LocalVariables|GetAllPawns)))
          (bind _returnvalue (Game|SpawnActorfromClass "/Game/Blueprints/JamOtherPawn.JamOtherPawn_C" (Math|Transform|MakeTransform _location "0, 0, 0" "1,1,1") "AlwaysSpawn" 0 (Math|Integer|SelectInt (Math|Random|RandomIntegerinRange 0 (LocalVariables|GetPlayerLevel)) (Math|Random|RandomIntegerinRange (+ (LocalVariables|GetPlayerLevel) 1) (Variables|Constants|GetMaxColorLevel)) (< _index (LocalVariables|GetPreyNeeded))) 0))
          (Utilities|Array|Add (LocalVariables|GetAllPawns) _returnvalue))))))

(fn PickSpawnLocation
  (params (Existing :type Array%20of%20Actor%20Object%20References))
  (LocalVariables|SetStuffToAvoid Existing)
  (for _index (range 0 20)
    (bind _output_get (LocalVariables|SetNewCandidate (* (* (Math|Random|RandomUnitVector) (Math|Float|Sqrt (Math|Random|RandomFloat))) (* (Variables|Constants|GetAreaRadius) 0.8))))
    (LocalVariables|SetNewCandidateClosestSquaredDistance 9e+06)
    (for _array_element (LocalVariables|GetStuffToAvoid)
      (LocalVariables|SetNewCandidateClosestSquaredDistance (Math|Float|Min(Float) (Class|KismetMathLibrary|VectorDistance2DSquared (Transformation|GetActorLocation _array_element) _output_get) (LocalVariables|GetNewCandidateClosestSquaredDistance))))
    (Utilities|Array|Add (LocalVariables|GetCandidateLocations) (LocalVariables|GetNewCandidate))
    (Utilities|Array|Add (LocalVariables|GetCandidateLocationSquaredDistances) (LocalVariables|GetNewCandidateClosestSquaredDistance)))
  (return (Utilities|Array|Get(acopy) (LocalVariables|GetCandidateLocations) (.IndexOfMaxValue (Math|Float|MaxOfFloatArray (LocalVariables|GetCandidateLocationSquaredDistances))))))

(fn NoteOtherPawnConsumed
  (params (Pawn :type Jam%20Other%20Pawn%20Object%20Reference))
  (if (Variables|GameState|GetHasFinishedTutorial)
    (Population|PopulateEnvironment)
    (bind _outactors (Actor|GetAllActorsOfClass "/Game/Blueprints/JamOtherPawn.JamOtherPawn_C"))
    (if (== (Utilities|Array|Length _outactors) 1) ; did we just consume the last other
      (CallFunction|End))
    (elif (> (Default|GetColorLevel (Variables|Default|GetPlayer)) 2)
      (Variables|GameState|SetHasFinishedTutorial true)
      (Utilities|Time|SetTimerbyFunctionName 0 "PopulateEnvironment" 1.0))))

(fn SelectNewOtherColorLevel
  (params (Existing :type Array%20of%20Jam%20Pawn%20Base%20Object%20References))
  (LocalVariables|SetPlayerLevel (Default|GetColorLevel (Variables|Default|GetPlayer)))
  (LocalVariables|SetClosestHigherLevel (Variables|Constants|GetMaxColorLevel))
  (for _array_element Existing
    (bind _asjam_other_pawn (Utilities|Casting|CastToJamOtherPawn _array_element))
    (if (<= (Default|GetColorLevel _asjam_other_pawn) (LocalVariables|GetPlayerLevel))
      (Math|Integer|IncrementInt (LocalVariables|GetAvailablePreyCount))
      (else
        (LocalVariables|SetHasAnyPredators true)
        (LocalVariables|SetClosestHigherLevel (Math|Integer|Min(Integer) (LocalVariables|GetClosestHigherLevel) (Default|GetColorLevel _asjam_other_pawn))))))
  (if (or (<= (- (LocalVariables|GetClosestHigherLevel) (LocalVariables|GetPlayerLevel)) (LocalVariables|GetAvailablePreyCount)) (not (LocalVariables|GetHasAnyPredators)))
    (return (Math|Random|RandomIntegerinRange (LocalVariables|GetPlayerLevel) (Variables|Constants|GetMaxColorLevel)))
    (else
      (return (Math|Random|RandomIntegerinRange 0 (LocalVariables|GetPlayerLevel))))))

(fn SpawnPlayerDamagedFragment
  (bind _player (Variables|Default|GetPlayer))
  (bind _outactors (Actor|GetAllActorsOfClass "/Game/Blueprints/JamPawnBase.JamPawnBase_C"))
  (bind _location (Population|PickSpawnLocation _outactors))
  (bind _returnvalue (Game|SpawnActorfromClass "/Game/Blueprints/JamOtherPawn.JamOtherPawn_C" (Math|Transform|MakeTransform _location "0, 0, 0" "1,1,1") "AlwaysSpawn" 0 0 0))
  (Default|SetupasFragment _returnvalue)
  (Utilities|FlowControl|Sequence
    (:then_0
      (bind _returnvalue_2 (Niagara|SpawnSystemAttached "/Game/Effects/BurstSystem.BurstSystem" (Variables|/Game/Blueprints/JamPawnBase.JamPawnBase_C|GetDefaultSceneRoot _returnvalue) "None" "0, 0, 0" "0, 0, 0" "SnapToTargetIncludingScale" true true "AutoRelease" false))
      (Niagara|SetNiagaraVariable(Vector3) _returnvalue_2 "SourceLocation" (Transformation|GetActorLocation _player))
      (bind _color (Default|ColorforLevel _player (+ (Default|GetColorLevel _player) 1)))
      (Niagara|SetNiagaraVariable(LinearColor) _returnvalue_2 "SourceColor" _color)
      (bind _color_2 (Default|ColorforLevel _returnvalue 1))
      (Niagara|SetNiagaraVariable(LinearColor) _returnvalue_2 "TargetColor" _color_2)
      (Niagara|SetNiagaraVariable(Float) _returnvalue_2 "AdditionalLifetime" 0.5))
    (:then_1
      (Population|PopulateEnvironment))))

(fn SetupTutorial
  (LocalVariables|SetPawns (Utilities|Array|MakeArray (Variables|Default|GetPlayer)))
  (for _array_element (LocalVariables|GetLevels)
    (bind _location (Population|PickSpawnLocation (LocalVariables|GetPawns)))
    (bind _returnvalue (Game|SpawnActorfromClass "/Game/Blueprints/JamOtherPawn.JamOtherPawn_C" (Math|Transform|MakeTransform _location "0, 0, 0" "1,1,1") "AlwaysSpawn" 0 _array_element 0))
    (Utilities|Array|Add (LocalVariables|GetPawns) _returnvalue))
  (Variables|GameState|SetHasFinishedTutorial false))

(fn GetDesiredPopulation
  (bind _player (Variables|Default|GetPlayer))
  (bind _level (Default|GetColorLevel _player))
  (return (Math|Integer|SelectInt 4 (Math|Integer|SelectInt 5 7 (< _level 8)) (< _level 4))))

(fn End
  (bind _asjam_player_controller (Utilities|Casting|CastToJamPlayerController (Game|GetPlayerController 0)))
  (Variables|/Game/Blueprints/JamPlayerController.JamPlayerController_C|SetShouldObeyUserInput _asjam_player_controller false)
  (Variables|GameState|SetGameOver true)
  (Variables|GameState|SetPlaying false)
  (Widget|SetVisibility (Variables|UI|GetEndScreenWidget) "Visible"))