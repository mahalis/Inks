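; Player controller that moves the controlled pawn toward the mouse cursor, with axis inputs for world X/Y movement and Escape to quit.
; Every tick, DoMouseFollowing deprojects the cursor and intersects that ray with a horizontal plane at world zero to find a target point.
; It adds movement input toward that point, scaled down as the XY distance shrinks so the pawn eases in under the cursor.
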(event EventBeginPlay)

(event EventTick
  (params (DeltaSeconds :type Float%20%28single-precision%29))
  (CallFunction|DoMouseFollowing))

(event Input|AxisEvents|InputAxisMoveRight
  (params (AxisValue :type Float%20%28single-precision%29))
  (Pawn|Input|AddMovementInput (Pawn|GetControlledPawn) (Math|Vector|MakeVector 0.0 1.0 0.0) AxisValue false))

(event Input|AxisEvents|InputAxisMoveForward
  (params (AxisValue :type Float%20%28single-precision%29))
  (Pawn|Input|AddMovementInput (Pawn|GetControlledPawn) (Math|Vector|MakeVector 1.0 0.0 0.0) AxisValue false))

(event Input|KeyboardEvents|Escape
  (params (Key :type Key%20Structure :default "None"))
  (:Pressed
    (Game|QuitGame 0 "Quit" false)))

(fn ConstructionScript)

(fn DoMouseFollowing
  (bind _returnvalue (Pawn|GetControlledPawn))
  (bind (_locationx _locationy _returnvalue_2) (Game|Player|GetMousePosition))
  (bind _self self)
  (bind _returnvalue_3 (Transformation|GetActorLocation _returnvalue))
  (bind (_worldposition _worlddirection _returnvalue_4) (Class|GameplayStatics|DeprojectScreentoWorld _self (Math|Vector2D|MakeVector2D _locationx _locationy)))
  (bind _returnvalue_5 (* _worlddirection 2e+03))
  (bind _returnvalue_6 (+ _worldposition _returnvalue_5))
  (bind (_t _intersection _returnvalue_7) (Class|KismetMathLibrary|LinePlaneIntersectionOriginNormal _worldposition _returnvalue_6 "0, 0, 0" "0, 0,1.000000"))
  (bind _returnvalue_8 (- _intersection _returnvalue_3))
  (if (Math|Boolean|ANDBoolean _returnvalue_4 _returnvalue_7 _returnvalue_2)
    (bind _output_get (LocalVariables|SetDistanceFromCursor (Math|Vector|VectorLengthXY _returnvalue_8)))
    (Pawn|Input|AddMovementInput _returnvalue (Math|Vector|SelectVector "0, 0, 0" (/ _returnvalue_8 _output_get) (< _output_get 0.01)) (Math|Float|MapRangeClamped _output_get 0.0 5e+01 0.0 1.0) false)))