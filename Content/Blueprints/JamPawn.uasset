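; JamPawn is a pawn with floating movement that keeps itself inside a circular area around the world origin.
; Each tick, ClampToArea checks horizontal distance against a threshold just inside AreaRadius.
; When the pawn is past it and moving outward, its velocity is reflected about the direction from the center.
; If it is possessed by an OtherController, that controller is notified of the wall hit with that direction.
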(event EventBeginPlay)

(event Collision|EventActorBeginOverlap
  (params (OtherActor :type Actor%20Object%20Reference)))

(event EventTick
  (params (DeltaSeconds :type Float%20%28single-precision%29))
  (CallFunction|ClamptoArea))

(fn ConstructionScript)

(fn ClamptoArea
  (bind _returnvalue (Transformation|GetActorLocation))
  (bind _floatingpawnmovement (Variables|Default|GetFloatingPawnMovement))
  (bind _output_get (LocalVariables|SetDistanceFromCenter (Math|Vector|VectorLengthXY _returnvalue)))
  (if (> _output_get (* (Variables|Default|GetAreaRadius) 0.98))
    (bind _output_get_2 (LocalVariables|SetDirectionFromCenter (/ _returnvalue (LocalVariables|GetDistanceFromCenter))))
    (if (> (Math|Vector|DotProduct (Variables|/Script/Engine.MovementComponent|GetVelocity _floatingpawnmovement) _output_get_2) 0.0)
      (Variables|/Script/Engine.MovementComponent|SetVelocity _floatingpawnmovement (- (Variables|/Script/Engine.MovementComponent|GetVelocity _floatingpawnmovement) (* _output_get_2 (* 2.0 (Math|Vector|DotProduct (Variables|/Script/Engine.MovementComponent|GetVelocity _floatingpawnmovement) _output_get_2)))))
      (bind _asother_controller (Utilities|Casting|CastToOtherController (Pawn|GetController)))
      (Default|NotifyHitWall _asother_controller (LocalVariables|GetDirectionFromCenter)))))