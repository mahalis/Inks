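; Base pawn for a game jam arena game where spheres carry a color level and react to touching paler pawns.
; A random starting level drives the saturation of the sphere's dynamic material, keeping the base hue and value.
; Overlapping a pawn of equal or lower level calls HandleHitPaler, empty here.
; Each tick, outward velocity is reflected near the circular area's edge, and an OtherController, if possessing, is notified of the wall hit.
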(event EventBeginPlay
  (bind _sphere (Variables|Default|GetSphere))
  (bind _returnvalue (Rendering|Material|CreateDynamicMaterialInstance _sphere 0 (Rendering|Material|GetMaterial _sphere 0) "None" :!class /Script/Engine.PrimitiveComponent))
  (bind _output_get (Variables|Default|SetMaterialInstance _returnvalue))
  (Rendering|Material|SetMaterial (Variables|Default|GetSphere) 0 _output_get)
  (bind _returnvalue_2 (Rendering|Material|GetVectorParameterValue _output_get "Color" :!class /Script/Engine.MaterialInstanceDynamic))
  (Variables|Default|SetBaseColor _returnvalue_2)
  (CallFunction|SetColorLevel (Math|Random|RandomIntegerinRange 0 5)))

(event Collision|EventActorBeginOverlap
  (params (OtherActor :type Actor%20Object%20Reference))
  (bind _asjam_pawn_base (Utilities|Casting|CastToJamPawnBase OtherActor))
  (if (<= (CallFunction|GetColorLevel _asjam_pawn_base) (Variables|Default|GetColorLevel))
    (CallFunction|HandleHitPaler _asjam_pawn_base)))

(event EventTick
  (params (DeltaSeconds :type Float%20%28single-precision%29))
  (CallFunction|ClamptoArea))

(fn ConstructionScript)

(fn ClamptoArea
  (bind _returnvalue (Transformation|GetActorLocation))
  (bind _floatingpawnmovement (Variables|Default|GetFloatingPawnMovement))
  (bind _output_get (LocalVariables|SetDistanceFromCenter (Math|Vector|VectorLengthXY _returnvalue)))
  (if (> _output_get (* (Variables|Default|GetAreaRadius) 0.98))
    (bind _output_get_2 (LocalVariables|SetDirectionFromCenter (/ _returnvalue (LocalVariables|GetDistanceFromCenter))))
    (if (> (Math|Vector|DotProduct (Variables|/Script/Engine.MovementComponent|GetVelocity _floatingpawnmovement) _output_get_2) 0.0)
      (Variables|/Script/Engine.MovementComponent|SetVelocity _floatingpawnmovement (- (Variables|/Script/Engine.MovementComponent|GetVelocity _floatingpawnmovement) (* _output_get_2 (* 2.0 (Math|Vector|DotProduct (Variables|/Script/Engine.MovementComponent|GetVelocity _floatingpawnmovement) _output_get_2)))))
      (bind _asother_controller (Utilities|Casting|CastToOtherController (Pawn|GetController)))
      (Default|NotifyHitWall _asother_controller (LocalVariables|GetDirectionFromCenter)))))

(fn GetColorLevel
  (return (Variables|Default|GetColorLevel)))

(fn SetColorLevel
  (params (Level :type Integer))
  (bind _basecolor (Variables|Default|GetBaseColor))
  (bind _returnvalue (Class|KismetMathLibrary|RGBLineartoHSV _basecolor))
  (bind _output_get (Variables|Default|SetColorLevel (Math|Integer|Min(Integer) Level (Variables|Default|GetMaxColorLevel))))
  (Rendering|Material|SetVectorParameterValue (Variables|Default|GetMaterialInstance) "Color" (Class|KismetMathLibrary|HSVtoRGBLinear (Utilities|Struct|MakeLinearColor (.r _returnvalue) (/ (Math|Conversions|ToFloat(Integer) (+ _output_get 1)) (Math|Conversions|ToFloat(Integer) (Variables|Default|GetMaxColorLevel))) (.b _returnvalue) 1.0)) :!class /Script/Engine.MaterialInstanceDynamic))

(fn HandleHitPaler
  (params (Other :type Jam%20Pawn%20Base%20Object%20Reference)))